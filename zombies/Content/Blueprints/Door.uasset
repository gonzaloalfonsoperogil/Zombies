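; Door is a double door actor that costs target points to open.
; ToggleDoor reads TargetScore from FirstPersonGameMode and, if it covers RequiredPoints, deducts that amount and hits a FlipFlop.
; The A branch plays two timelines that yaw the left and right pivots 90 degrees in opposite directions.
; The B branch is unwired, so alternate paid calls deduct points without animating, and no closing logic exists.
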(event `Toggle Door`
  (bind _required_points (`self.Required Points`))
  (bind _asfirst_person_game_mode (cast `/Game/FirstPersonBP/Blueprints/FirstPersonGameMode` (`GameplayStatics.GetGameMode`)))
  (if (>= (`/Game/FirstPersonBP/Blueprints/FirstPersonGameMode.TargetScore` _asfirst_person_game_mode) _required_points)
    (`/Game/FirstPersonBP/Blueprints/FirstPersonGameMode.RemoveTargetPoints` _asfirst_person_game_mode _required_points)
    (`/Engine/EditorBlueprintResources/StandardMacros.FlipFlop`
      (:`A`
        (`|ExecutionSequence`
          (:`then_0`
            (bind (_direction _alpha) (`Timeline|Left Door Lerp`)
              (:`Update`
                (`SceneComponent.K2_SetRelativeRotation` (`self.LeftPivot`) (`KismetMathLibrary.MakeRotator` 0.0 0.0 (`KismetMathLibrary.Lerp` 0.0 -90.0 _alpha)) false false))))
          (:`then_1`
            (bind (_direction_2 _alpha_2) (`Timeline|Right Door Lerp`)
              (:`Update`
                (`SceneComponent.K2_SetRelativeRotation` (`self.RightPivot`) (`KismetMathLibrary.MakeRotator` 0.0 0.0 (`KismetMathLibrary.Lerp` 0.0 90.0 _alpha_2)) false false)))))))))

(fn `UserConstructionScript`)